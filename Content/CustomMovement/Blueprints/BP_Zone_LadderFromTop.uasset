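; Ladder zone actor for the custom movement system that has top and middle entry but no bottom entry or exit.
; Its construction script spawns cube rungs from StepCount and StepHeight, then resizes the trigger and moves the Bottom marker to match.
; Trigger overlaps register the zone with BP_CustomMoveBaseCharacter.
; Enter and exit checks test distance to marker components and input strength, with entries also comparing input direction to ladder facing.
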(event `self.ReceiveBeginPlay`)

(event `self.TriggerBox.OnComponentBeginOverlap`
  (params (OverlappedComponent :type "PrimitiveComponent Object Reference") (OtherActor :type "Actor Object Reference") (OtherComp :type "PrimitiveComponent Object Reference") (OtherBodyIndex :type Integer) (bFromSweep :type Boolean) (SweepResult :type "HitResult Structure (by ref)"))
  (bind _asbp_custom_move_base_character (cast `/Game/CustomMovement/Blueprints/BP_CustomMoveBaseCharacter` OtherActor))
  (`/Game/CustomMovement/Blueprints/BP_CustomMoveBaseCharacter.BeginOverlappedCustomMoveZone` _asbp_custom_move_base_character (make `/Game/CustomMovement/Blueprints/SCustomMoveZone` self "NewEnumerator0")))

(event `self.TriggerBox.OnComponentEndOverlap`
  (params (OverlappedComponent :type "PrimitiveComponent Object Reference") (OtherActor :type "Actor Object Reference") (OtherComp :type "PrimitiveComponent Object Reference") (OtherBodyIndex :type Integer))
  (bind _asbp_custom_move_base_character (cast `/Game/CustomMovement/Blueprints/BP_CustomMoveBaseCharacter` OtherActor))
  (`/Game/CustomMovement/Blueprints/BP_CustomMoveBaseCharacter.EndOverlappedCustomMoveZone` _asbp_custom_move_base_character self))

(fn `CheckEnterToBottom`
  (params (`Character Bottom Location` :type "Vector Structure") (`Input Direction` :type "Vector Structure") (`Input Scale` :type "Float (double-precision)"))
  (returns (Result :type Boolean))
  (return false))

(fn `CheckEnterToMiddle`
  (params (`Character Bottom Location` :type "Vector Structure") (`Input Direction` :type "Vector Structure") (`Input Scale` :type "Float (double-precision)"))
  (returns (Result :type Boolean))
  (bind _returnvalue (`self.GetActorForwardVector`))
  (return (and (< (`KismetMathLibrary.VSize` (- `Character Bottom Location` (`SceneComponent.K2_GetComponentLocation` (`self.Bottom`)))) 50.0) (or (and (> `Input Scale` 0.8) (>= (`KismetMathLibrary.Dot_VectorVector` `Input Direction` _returnvalue) 0.7)) (and (<= (`KismetMathLibrary.Dot_VectorVector` _returnvalue `Input Direction`) -0.7) (< `Input Scale` -0.8))))))

(fn `CheckEnterToTop`
  (params (`Character Bottom Location` :type "Vector Structure") (`Input Direction` :type "Vector Structure") (`Input Scale` :type "Float (double-precision)"))
  (returns (Result :type Boolean))
  (bind _returnvalue (`self.GetActorForwardVector`))
  (return (and (<= (`KismetMathLibrary.VSize` (- `Character Bottom Location` (`SceneComponent.K2_GetComponentLocation` (`self.Top_Enter`)))) 50.0) (or (and (> `Input Scale` 0.3) (<= (`KismetMathLibrary.Dot_VectorVector` `Input Direction` _returnvalue) -0.7)) (and (>= (`KismetMathLibrary.Dot_VectorVector` _returnvalue `Input Direction`) 0.7) (< `Input Scale` -0.3))))))

(fn `CheckExitToBottom`
  (params (`Character Bottom Location` :type "Vector Structure") (`Input Scale` :type "Float (double-precision)"))
  (returns (Result :type Boolean))
  (return false))

(fn `CheckExitToTop`
  (params (`Character Bottom Location` :type "Vector Structure") (`Input Scale` :type "Float (double-precision)"))
  (returns (Result :type Boolean))
  (return (and (> `Input Scale` 0.8) (<= (`KismetMathLibrary.VSize` (- `Character Bottom Location` (`SceneComponent.K2_GetComponentLocation` (`self.Top`)))) 1.0))))

(fn `GetLadderLocation`
  (returns (`Top Location` :type "Vector Structure") (`Bottom Location` :type "Vector Structure"))
  (return (`SceneComponent.K2_GetComponentLocation` (`self.Top`)) (`SceneComponent.K2_GetComponentLocation` (`self.Bottom`))))

(fn `GetLadderRotation`
  (returns (`Ladder Rotation` :type "Rotator Structure"))
  (return (`self.K2_GetActorRotation`)))

(fn `GetLadderStepHeight`
  (returns (StepHeight :type "Float (double-precision)"))
  (return (`self.Step Height`)))

(fn `GetTopEnterLocation`
  (returns (`Top Enter Location` :type "Vector Structure"))
  (return (`SceneComponent.K2_GetComponentLocation` (`self.Top_Enter`))))

(fn `UserConstructionScript`
  (bind _triggerbox (`self.TriggerBox`))
  (bind _triggerbox_2 (`self.TriggerBox`))
  (bind _bottom (`self.Bottom`))
  (bind (_relativescale3d_x _relativescale3d_y _relativescale3d_z) (`KismetMathLibrary.BreakVector` (`SceneComponent.RelativeScale3D` _triggerbox)))
  (bind (_relativelocation_x _relativelocation_y) (`KismetMathLibrary.BreakVector` (`SceneComponent.RelativeLocation` _triggerbox_2)))
  (bind (_relativelocation_x_2 _relativelocation_y_2 _relativelocation_z) (`KismetMathLibrary.BreakVector` (`SceneComponent.RelativeLocation` _bottom)))
  (bind _returnvalue (/ (`KismetMathLibrary.Conv_IntToDouble` (+ (`self.Step Count`) 3)) 4.0))
  (`SceneComponent.SetRelativeScale3D` _triggerbox (`KismetMathLibrary.MakeVector` _relativescale3d_x _relativescale3d_y (* (+ _relativescale3d_z (/ 0.5 _returnvalue)) _returnvalue)))
  (`SceneComponent.K2_SetRelativeLocation` _triggerbox_2 (`KismetMathLibrary.MakeVector` _relativelocation_x _relativelocation_y (- (.z (`.BoxExtent` (`KismetSystemLibrary.GetComponentBounds` _triggerbox_2))) (* (- (`self.Step Count`) 1) (`self.Step Height`)))) false false)
  (`SceneComponent.K2_SetRelativeLocation` _bottom (`KismetMathLibrary.MakeVector` _relativelocation_x_2 _relativelocation_y_2 (- _relativelocation_z (* (- (`self.Step Count`) 1) (`self.Step Height`)))) false false)
  (for _index (range (`self.Step Count`))
    (bind _returnvalue_2 (`AddComponent|NODE_AddStaticMeshComponent-1` :`RelativeTransform` (`KismetMathLibrary.MakeTransform` (`KismetMathLibrary.MakeVector` 0.0 0.0 (* (- 4 _index) (`self.Step Height`))) (struct) (0.05 1.0 0.05))))
    (`StaticMeshComponent.SetStaticMesh` _returnvalue_2 "/Game/CustomMovement/Meshes/SM_Cube.SM_Cube")))